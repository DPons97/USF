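; BP_TimewarsPlayerController is the Timewars player controller that spawns units at the mouse cursor when Spacebar is pressed.
; A visibility trace under the cursor supplies the location to AddUnitEvent.
; That event has BP_TimewarsGameMode spawn the unit with the Timewars pawn as owner, then inserts it at the front of the TimewarsPlayerState's UnitsList.
; The construction script and NewFunction_0 are empty.
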(event Custom|AddUnitEvent
  (params (SpawnLocation :type Vector))
  (bind _asbp_timewars_game_mode (Utilities|Casting|CastToBP_TimewarsGameMode (Game|GetGameMode)))
  (bind _spawnedunit (Default|SpawnUnit _asbp_timewars_game_mode SpawnLocation (Class|TimewarsPlayerController|GetTimewarsPawn)))
  (bind _astimewars_player_state (Utilities|Casting|CastToTimewarsPlayerState (Variables|Default|GetPlayerState)))
  (Utilities|Array|Insert (Variables|/Script/Project_Timewars.TimewarsPlayerState|GetUnitsList _astimewars_player_state) _spawnedunit))

(event Input|ActionEvents|InputActionSpacebar
  (params (Key :type Key%20Structure :default "None"))
  (:Pressed
    (CallFunction|AddUnitEvent (.Location (Collision|BreakHitResult (.HitResult (Game|Player|GetHitResultUnderCursorbyChannel "TraceTypeQuery1" true)))))))

(fn ConstructionScript)

(fn NewFunction0)